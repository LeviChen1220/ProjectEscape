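; Enemy spawner Blueprint that places AI enemy pawns at a set of spawn point actors.
; Its Spawn event async-loads EnemyCharacterClass, casts it to a Pawn class and spawns one AI at each SpawnPoints location, with NoCollisionFail set.
; The TriggerBox overlap handler is empty; the once-only survivor check that would call Spawn is disconnected, so nothing in this Blueprint triggers spawning.
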(event OnActorBeginOverlap(TriggerBox)
  (params (OverlappedActor :type Actor%20Object%20Reference) (OtherActor :type Actor%20Object%20Reference)))

(event Custom|Spawn
  (bind _spawnpoints (Variables|Default|GetSpawnPoints))
  (bind _class (Utilities|AsyncLoadClassAsset (Variables|Default|GetEnemyCharacterClass))
    (:Completed
      (bind _aspawn (Utilities|Casting|CastToPawnClass _class))
      (if (Utilities|Array|IsNotEmpty _spawnpoints)
        (for _array_element _spawnpoints
          (AI|SpawnAIFromClass _aspawn 0 (Transformation|GetActorLocation _array_element) "0, 0, 0" true 0))))))

(event EventBeginPlay)

(event Collision|EventActorBeginOverlap
  (params (OtherActor :type Actor%20Object%20Reference)))

(event EventTick
  (params (DeltaSeconds :type Float%20%28single-precision%29)))

(fn ConstructionScript)